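; VR shooter player character that extends a parent pawn with health, cooldown-limited teleporting and hand-based UI interaction.
; Teleport events reach the parent only off cooldown, while Tick updates the cooldown and status text.
; Damage flashes the screen; death disables input, fades the view and reopens the current level as a listen server.
; Healing potion pickup is authority-only, and an active UI hand forwards grab and key input to widget interaction.
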(event `self.ReceiveBeginPlay`
  (`parent.ReceiveBeginPlay`)
  (set `/Game/Shooter/GUI/PlayerStatusBar.Character` self (cast `/Game/Shooter/GUI/PlayerStatusBar` (`WidgetComponent.GetUserWidgetObject` (`self.Widget`)) :!pure true)))

(event `self.ReceiveTick`
  (params (DeltaSeconds :type "Float (single-precision)"))
  (`parent.ReceiveTick` DeltaSeconds)
  (`self.UpdateCooldown` DeltaSeconds)
  (`self.Update Text`))

(event `self.SetTeleporterActive`
  (params (Hand :type "EControllerHand Enum" :default "Left") (Active :type Boolean))
  (if (== (`self.CurrentTeleportCooldown`) 0.0)
    (`parent.SetTeleporterActive` Hand Active)
    (else
      (`parent.SetTeleporterActive` "Left" false)
      (`parent.SetTeleporterActive` "Right" false))))

(event `self.ExecuteTeleportation`
  (params (MotionController :type "/Game/VRExpansion/Vive/BP_Teleport_Controller Object Reference") (MovementMode :type "/Game/VRExpansion/Vive/MovementMode Enum" :default "NewEnumerator0") (Hand :type "EControllerHand Enum" :default "Left"))
  (if (== (`self.CurrentTeleportCooldown`) 0.0)
    (`parent.ExecuteTeleportation` MotionController MovementMode Hand)
    (set `self.CurrentTeleportCooldown` (`self.TeleportCooldown`))))

(event `InputAction|GrabRight` :overrideparent false
  (params (Key :type "Key Structure"))
  (bind _is_active_ui_hand (`self.Is Active UI Hand`))
  (bind _widgetinteraction (`self.WidgetInteraction`))
  ;[1 1 1] UI interactive
  (:`Pressed`
    (if _is_active_ui_hand
      (`WidgetInteractionComponent.PressPointerKey` _widgetinteraction "LeftMouseButton")))
  (:`Released`
    (if _is_active_ui_hand
      (`WidgetInteractionComponent.ReleasePointerKey` _widgetinteraction "LeftMouseButton"))))

(event `self.ReceiveAnyDamage`
  (params (Damage :type "Float (single-precision)") (DamageType :type "DamageType Object Reference") (InstigatedBy :type "Controller Object Reference") (DamageCauser :type "Actor Object Reference"))
  (`parent.ReceiveAnyDamage` Damage DamageType InstigatedBy DamageCauser)
  (if (not (`self.IsDie`))
    (`self.On Damaged` Damage)
    (bind _output_get (set `self.Health` (`KismetMathLibrary.FMax` (- (`self.Health`) Damage))))
    (if (== _output_get 0.0)
      (set `self.IsDie` true)
      (`self.On Die`)
      (`KismetSystemLibrary.Delay` 1.0)
      (bind _returnvalue (`GameplayStatics.GetCurrentLevelName` true))
      (`GameplayStatics.OpenLevel` (`KismetStringLibrary.Conv_StringToName` _returnvalue) true "listen"))))

(event `Key|AnyKey`
  (params (Key :type "Key Structure"))
  (bind _widgetinteraction (`self.WidgetInteraction`))
  (bind _is_active_ui_hand (`self.Is Active UI Hand`))
  ;[1 1 1] UI interactive
  (:`Pressed`
    (if _is_active_ui_hand
      (`WidgetInteractionComponent.PressKey` _widgetinteraction Key false)))
  (:`Released`
    (if _is_active_ui_hand
      (`WidgetInteractionComponent.ReleaseKey` _widgetinteraction Key))))

(event `On Die`
  (set `self.IsDie` true)
  (`self.DisableInput` (`GameplayStatics.GetPlayerController` 0))
  (`KismetSystemLibrary.PrintString` (`KismetTextLibrary.Conv_TextToString` (`|FormatText` "{0} has been killed" (`KismetTextLibrary.Conv_StringToText` (`KismetSystemLibrary.GetDisplayName` self)))))
  (if (`self.IsPlayerControlled`)
    (`PlayerCameraManager.StartCameraFade` (`GameplayStatics.GetPlayerCameraManager` (`AdvancedSessionsLibrary.GetNetPlayerIndex` null)) 0.0 0.9 0.2 (struct :`R` 0.020833) false true)))

(event `On Damaged`
  (params (Damage :type "Float (double-precision)"))
  (`PlayerCameraManager.StartCameraFade` (`GameplayStatics.GetPlayerCameraManager` (`AdvancedSessionsLibrary.GetNetPlayerIndex` null)) 0.3 0.0 0.2 (struct :`R` 0.020833) false true))

(event `self.PickUpCollision.OnComponentBeginOverlap`
  (params (OverlappedComponent :type "PrimitiveComponent Object Reference") (OtherActor :type "Actor Object Reference") (OtherComp :type "PrimitiveComponent Object Reference") (OtherBodyIndex :type Integer) (bFromSweep :type Boolean) (SweepResult :type "HitResult Structure (by ref)"))
  (`/Engine/EditorBlueprintResources/ActorMacros.Switch Has Authority`
    (:`Authority`
      (bind _asheal_potion (cast `/Game/Shooter/Blueprints/HealPotion` OtherActor))
      (if (< (`self.Health`) (`self.MaxHealth`))
        (set `self.Health` (`KismetMathLibrary.FMin` (`KismetMathLibrary.FMax` (+ (`/Game/Shooter/Blueprints/HealPotion.Heal Value` _asheal_potion) (`self.Health`))) (`self.MaxHealth`)))
        (`self.K2_DestroyActor` _asheal_potion)))))

(fn `SetActiveUiHand`
  (params (`Is Active` :type Boolean))
  (bind _widgetinteraction (`self.WidgetInteraction`))
  (bind _output_get (set `self.Is Active UI Hand` `Is Active`))
  (`ActorComponent.SetActive` _widgetinteraction _output_get false)
  (`SceneComponent.SetVisibility` _widgetinteraction _output_get false)
  (set `WidgetInteractionComponent.bEnableHitTesting` _output_get _widgetinteraction))

(fn `Update Text`
  (bind _currentteleportcooldown (`self.CurrentTeleportCooldown`))
  (bind _teleportcooldowntext (`self.TeleportCooldownText`))
  (`TextRenderComponent.K2_SetText` (`self.HealthText`) (`KismetTextLibrary.Conv_DoubleToText` (`self.Health`) "HalfToEven"))
  (`TextRenderComponent.K2_SetText` _teleportcooldowntext (`KismetTextLibrary.Conv_DoubleToText` _currentteleportcooldown "HalfToEven" false true 1 324 2 2))
  (`SceneComponent.SetVisibility` _teleportcooldowntext (!= _currentteleportcooldown 0.0) false))

(fn `UpdateCooldown`
  (params (DeltaTime :type "Float (double-precision)"))
  (set `self.CurrentTeleportCooldown` (`KismetMathLibrary.FMax` (- (`self.CurrentTeleportCooldown`) DeltaTime)))
  (return))

(fn `UserConstructionScript`
  (`parent.UserConstructionScript`)
  (set `self.Health` (`self.MaxHealth`)))