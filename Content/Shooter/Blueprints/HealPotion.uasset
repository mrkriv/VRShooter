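; HealPotion is an actor that animates a potion with a spinning and bobbing idle motion; the graph holds no healing or pickup logic.
; Each tick it yaws the whole actor at RotationSpeed scaled by delta time.
; It accumulates time and moves the Cube component along Z with a sine wave driven by MoveSpeed and MoveRange.
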(event `self.ReceiveTick`
  (params (DeltaSeconds :type "Float (single-precision)"))
  (set `self.Time` (+ DeltaSeconds (`self.Time`)))
  (`self.K2_AddActorWorldRotation` (`KismetMathLibrary.MakeRotator` 0.0 0.0 (* DeltaSeconds (`self.Rotation Speed`))))
  (`SceneComponent.K2_SetRelativeLocation` (`self.Cube`) (`KismetMathLibrary.MakeVector` 0.0 0.0 (* (`KismetMathLibrary.Sin` (* (`self.Time`) (`self.Move Speed`))) (`self.Move Range`))) false false))

(fn `UserConstructionScript`)