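; GameInformer is a pre-round gate actor that starts a countdown once all its assigned buttons have been pressed.
; Button presses are forwarded to a server event, which records each button and destroys it on authority after a short delay.
; When the ready count matches the button count, Tick counts StartTime down on two info texts.
; At zero, it hides the root with its children and disables the Box collision.
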(event `self.ReceiveBeginPlay`
  (for _array_element (`self.Buttons`)
    (add `/Game/VRExpansion/Button/ButtonActor.ButtonPressed` _array_element (delegate `OnButtonClicked`))))

(event `OnButtonClicked`
  (params (Sender :type "/Game/VRExpansion/Button/ButtonActor Object Reference"))
  (`self.OnButtonClicked_Server` Sender))

(event `OnButtonClicked_Server`
  (params (Button :type "Actor Object Reference (by ref)"))
  (bind _ready_buttons (`self.Ready Buttons`))
  (`BlueprintSetLibrary.Set_Add` _ready_buttons Button)
  (`|ExecutionSequence`
    (:`then_0`
      (`/Engine/EditorBlueprintResources/ActorMacros.Switch Has Authority`
        (:`Authority`
          (`KismetSystemLibrary.Delay` 0.3)
          (`self.K2_DestroyActor` Button))))
    (:`then_1`
      (if (== (`BlueprintSetLibrary.Set_Length` _ready_buttons) (`KismetArrayLibrary.Array_Length` (`self.Buttons`)))
        (`self.Begin Start Round`)))))

(event `Begin Start Round`
  (set `self.Begin Start` true))

(event `self.ReceiveTick`
  (params (DeltaSeconds :type "Float (single-precision)"))
  (if (`self.Begin Start`)
    (bind _output_get (set `self.Start Time` (`KismetMathLibrary.FMax` (- (`self.Start Time`) DeltaSeconds))))
    (`TextRenderComponent.K2_SetText` (`self.InfoText1`) (`KismetTextLibrary.Conv_DoubleToText` _output_get "HalfToEven" false true 1 324 1 1))
    (`TextRenderComponent.K2_SetText` (`self.InfoText2`) (`KismetTextLibrary.Conv_DoubleToText` _output_get "HalfToEven" false true 1 324 1 1))
    (if (== (`self.Start Time`) 0.0)
      (set `self.Begin Start` false)
      (`self.Start Round`))))

(event `Start Round`
  (`SceneComponent.SetVisibility` (`self.DefaultSceneRoot`) false true)
  (`PrimitiveComponent.SetCollisionEnabled` (`self.Box`) "NoCollision"))

(fn `UserConstructionScript`)